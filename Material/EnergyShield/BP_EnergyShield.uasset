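; BP_EnergyShield is an energy shield actor whose dissolve effect responds to the player entering or leaving a trigger box.
; Overlaps on CollisionTestBox, matched by the display name "ThirdPersonCharacter", play or reverse the ShieldClose timeline and track InCollision.
; The timeline drives DissolveUpPos in the shared MC_Shield material parameter collection, initialized at BeginPlay.
; ManualShieldIn and ManualShieldOut reverse or play that timeline while InCollision is true.
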(event `self.ReceiveBeginPlay`
  (`|ExecutionSequence`
    (:`then_0`
      (`KismetMaterialLibrary.SetScalarParameterValue` "/Game/Shader/ShaderLib_Privacy/Material/EnergyShield/MC_Shield.MC_Shield" "DissolveUpPos" 1.2))))

(event `self.CollisionTestBox.OnComponentBeginOverlap`
  (params (OverlappedComponent :type "PrimitiveComponent Object Reference") (OtherActor :type "Actor Object Reference") (OtherComp :type "PrimitiveComponent Object Reference") (OtherBodyIndex :type Integer) (bFromSweep :type Boolean) (SweepResult :type "HitResult Structure (by ref)"))
  (`|ExecutionSequence`
    (:`then_0`
      (if (`KismetStringLibrary.EqualEqual_StrStr` (`KismetSystemLibrary.GetDisplayName` OtherActor) "ThirdPersonCharacter")
        (set `self.InCollision?` true)))
    (:`then_1`
      (if (`self.InCollision?`)
        (bind (_direction _newtrack_0) (`Timeline|ShieldClose` :!label _label)
          (:`Update`
            (`KismetMaterialLibrary.SetScalarParameterValue` "/Game/Shader/ShaderLib_Privacy/Material/EnergyShield/MC_Shield.MC_Shield" "DissolveUpPos" _newtrack_0)))))))

(event `ManualShieldIn`
  (if (`self.InCollision?`)
    (goto _label :!via `Reverse`)))

(event `ManualShieldOut`
  (if (`self.InCollision?`)
    (goto _label)))

(event `self.CollisionTestBox.OnComponentEndOverlap`
  (params (OverlappedComponent :type "PrimitiveComponent Object Reference") (OtherActor :type "Actor Object Reference") (OtherComp :type "PrimitiveComponent Object Reference") (OtherBodyIndex :type Integer))
  (if (`KismetStringLibrary.EqualEqual_StrStr` (`KismetSystemLibrary.GetDisplayName` OtherActor) "ThirdPersonCharacter")
    (`|ExecutionSequence`
      (:`then_0`
        (goto _label :!via `Reverse`))
      (:`then_1`
        (set `self.InCollision?` false)))))

(fn `UserConstructionScript`)