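; BP_PortalManagement links the Magic and Heal actors as a two-way portal pair for the player pawn.
; Every Tick it checks whether the pawn overlaps either actor, then teleports it to the other's location while keeping its rotation.
; A shared MagicHealCanTele flag turns off for two seconds after each jump, preventing an immediate bounce back.
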(event `self.ReceiveTick`
  (params (DeltaSeconds :type "Float (single-precision)"))
  (bind _returnvalue (`GameplayStatics.GetPlayerPawn` 0))
  (bind _returnvalue_2 (`GameplayStatics.GetPlayerPawn` 0))
  (`|ExecutionSequence`
    (:`then_0`
      (if (`self.IsOverlappingActor` (`self.Magic`) _returnvalue_2)
        (if (`self.Magic_Heal_CanTele`)
          (`self.K2_TeleportTo` _returnvalue_2 (`SceneComponent.K2_GetComponentLocation` (`Actor.RootComponent` (`self.Heal`))) (`self.K2_GetActorRotation` _returnvalue_2))
          (set `self.Magic_Heal_CanTele` false)
          (`KismetSystemLibrary.Delay` 2.0)
          (set `self.Magic_Heal_CanTele` true))
        (elif (`self.IsOverlappingActor` (`self.Heal`) _returnvalue)
          (if (`self.Magic_Heal_CanTele`)
            (`self.K2_TeleportTo` _returnvalue (`SceneComponent.K2_GetComponentLocation` (`Actor.RootComponent` (`self.Magic`))) (`self.K2_GetActorRotation` _returnvalue))
            (set `self.Magic_Heal_CanTele` false)
            (`KismetSystemLibrary.Delay` 2.0)
            (set `self.Magic_Heal_CanTele` true)))))))

(fn `UserConstructionScript`)